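; Detached player camera pawn that cycles between free, angled top follow and level side follow views of the Player_Troll character.
; A DoN counter on CameraAction steps through the modes, toggling follow and swapping camera rotation and follow offset.
; Tick either snaps the pawn to the troll plus offset or edge-scrolls it with movement input when the cursor passes viewport margins computed at BeginPlay.
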(event EventBeginPlay
  (CallFunction|GetPlayerCharacterRef)
  (Variables|Default|SetCameraFollowOffset (Variables|Setup|GetTop_CameraFollowOffset))
  (CallFunction|UpdateCameraPosition)
  (CallFunction|SetXandYBounds)
  (Variables|/Script/Engine.PlayerController|SetbShowMouseCursor (Game|GetPlayerController 0) true))

(event EventTick
  (params (DeltaSeconds :type Float%20%28single-precision%29))
  ;[1 1 1] Camera follows on tick if its turned on
  (if (Variables|Default|GetbIsFollowing)
    (CallFunction|UpdateCameraPosition)
    (else
      (CallFunction|HandleEdgeScroll))))

(event Input|ActionEvents|InputActionCameraAction
  (params (Key :type Key%20Structure :default "AnyKey"))
  ;[1 1 1] Pawn has 3 camera modes: free, follow 45', follow 0'
  (:Pressed
    (bind _counter (Utilities|FlowControl|DoN 3 :!label _label)
      (:Exit
        (switch int _counter
          (:1
            (CallFunction|ToggleFollow))
          (:2
            (CallFunction|SetSideFollow))
          (:3
            (CallFunction|SetTopFreeCamera)
            (goto _label Reset)))))))

(fn ConstructionScript)

(fn GetPlayerCharacterRef
  (bind _outactors (Actor|GetAllActorsOfClass "/Game/Player/Player_Troll/Player_Troll.Player_Troll_C"))
  (Variables|Default|SetPlayerCharacterRef (Utilities|Array|Get(acopy) _outactors)))

(fn UpdateCameraPosition
  (Transformation|SetActorLocation (+ (Transformation|GetActorLocation (Variables|Default|GetPlayerCharacterRef)) (Variables|Default|GetCameraFollowOffset)) false false))

(fn ToggleFollow
  (if (Variables|Default|GetbIsFollowing)
    (Variables|Default|SetbIsFollowing false)
    (else
      (Variables|Default|SetbIsFollowing true))))

(fn SetXandYBounds
  (bind _returnvalue (Viewport|GetViewportSize))
  (bind _mousescrollscreenboundpercentage (Variables|Setup|GetMouseScrollScreenBoundPercentage))
  (bind _returnvalue_2 (/ (.x _returnvalue) _mousescrollscreenboundpercentage))
  (bind _returnvalue_3 (/ (.y _returnvalue) _mousescrollscreenboundpercentage))
  (Variables|Default|SetXMin _returnvalue_2)
  (Variables|Default|SetXMax (- (.x _returnvalue) _returnvalue_2))
  (Variables|Default|SetYMin _returnvalue_3)
  (Variables|Default|SetYMax (- (.y _returnvalue) _returnvalue_3)))

(fn GetScrollAxis
  (params (Input :type Float%20%28single-precision%29) (Min :type Float%20%28single-precision%29) (Max :type Float%20%28single-precision%29))
  (LocalVariables|SetOutAxis 0.0)
  (Utilities|FlowControl|Sequence
    (:then_0
      (Math|Float|CompareFloat Input Min
        (:<
          (LocalVariables|SetOutAxis -1.0))))
    (:then_1
      (Math|Float|CompareFloat Input Max
        (:>
          (LocalVariables|SetOutAxis 1.0))))
    (:then_2
      (return (LocalVariables|GetOutAxis)))))

(fn HandleXScroll
  (params (Input :type Float%20%28single-precision%29))
  (bind _axistomove (CallFunction|GetScrollAxis Input (Variables|Default|GetXMin) (Variables|Default|GetXMax)))
  (Pawn|Input|AddMovementInput (Math|Vector|GetRightVector (Transformation|GetActorRotation)) _axistomove false))

(fn HandleYScroll
  (params (Input :type Float%20%28single-precision%29))
  (bind _axistomove (CallFunction|GetScrollAxis Input (Variables|Default|GetYMin) (Variables|Default|GetYMax)))
  (Pawn|Input|AddMovementInput (Math|Vector|GetForwardVector (Transformation|GetActorRotation)) (* _axistomove -1.0) false))

(fn HandleEdgeScroll
  (bind _returnvalue (Game|GetPlayerController 0))
  (bind (_locationx _locationy) (Game|Player|GetMousePosition _returnvalue))
  (Utilities|FlowControl|Sequence
    (:then_0
      (CallFunction|HandleXScroll _locationx))
    (:then_1
      (CallFunction|HandleYScroll _locationy))))

(fn SetTopFreeCamera
  (CallFunction|ToggleFollow)
  (Transformation|SetRelativeRotation (Variables|Default|GetCamera) "-45.000000,0.000000,0.000000" false false)
  (Variables|Default|SetCameraFollowOffset (Variables|Setup|GetTop_CameraFollowOffset))
  (CallFunction|UpdateCameraPosition))

(fn SetSideFollow
  (Transformation|SetRelativeRotation (Variables|Default|GetCamera) "0.000000,0.000000,0.000000" false false)
  (Variables|Default|SetCameraFollowOffset (Variables|Setup|GetSide_CameraFollowOffset)))