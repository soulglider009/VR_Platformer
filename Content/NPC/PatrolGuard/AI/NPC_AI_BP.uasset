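; AI controller for the patrol guard NPC that starts its blackboard and behavior tree on BeginPlay.
; Perception updates for actors tagged "player" call SeePlayer on the guard and store the actor in the blackboard's enemy key, clearing it when sensing fails.
; Helpers SetFocalPoint, which writes the player pawn to that key rather than setting focus, and a debug perception printer are not called in this graph.
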(event OnTargetPerceptionUpdated(AIPerception)
  (params (Actor :type Actor%20Object%20Reference) (Stimulus :type AI%20Stimulus%20Structure))
  (bind _output_get (Variables|Default|SetSensedActor Actor))
  (if (Actor|ActorHasTag _output_get "player")
    (if (.bSuccessfullySensed (Utilities|Struct|BreakAIStimulus Stimulus))
      (bind _aspatrol_guard (Utilities|Casting|CastToPatrolGuard (Pawn|GetControlledPawn))
        (:then
          (Class|PatrolGuard|SeePlayer _aspatrol_guard)
          (CallFunction|AddSensedEnemytoBlackboard (Variables|Default|GetSensedActor)))
        (:CastFailed
          (Development|PrintString "Failed to cast to patrol guard")))
      (else
        (AI|Components|Blackboard|ClearValue (Variables|Default|GetBlackboardComp) (Variables|Default|GetEnemyKey))))))

(event EventBeginPlay
  (bind _blackboardcomponent (Class|AIController|UseBlackboard "/Game/NPC/PatrolGuard/AI/GuardData.GuardData"))
  (AI|RunBehaviorTree "/Game/NPC/PatrolGuard/AI/GuardBehavior.GuardBehavior")
  (Variables|Default|SetBlackboardComp _blackboardcomponent))

(fn ConstructionScript)

(fn PrintPerception
  (params (Object :type Object%20Object%20Reference) (Stimulus :type AI%20Stimulus%20Structure%20%28by%20ref%29))
  (bind _returnvalue (Class|AIPerceptionSystem|GetSenseClassforStimulus Stimulus))
  (Development|PrintString (Utilities|String|Append (Utilities|GetObjectName (Pawn|GetControlledPawn)) " " (Utilities|GetClassDisplayName _returnvalue) " " (Utilities|GetObjectName Object))))

(fn SetFocalPoint
  (params (Blackboard :type Blackboard%20Component%20Object%20Reference))
  (AI|Components|Blackboard|SetValueasObject Blackboard (Utilities|Name|MakeLiteralName (Variables|Default|GetEnemyKey)) (Game|Player|GetPlayerPawn 0)))

(fn AddSensedEnemytoBlackboard
  (params (ObjectValue :type Object%20Object%20Reference))
  (AI|Components|Blackboard|SetValueasObject (Variables|Default|GetBlackboardComp) (Utilities|Name|MakeLiteralName (Variables|Default|GetEnemyKey)) ObjectValue)
  (return))